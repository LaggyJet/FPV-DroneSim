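; BP_Wall_Paint_Decal is a configurable decal actor, apparently for painted wall detail in the Downtown Alley environment.
; Its construction script applies the chosen decal material, wraps it in a dynamic material instance and sets the decal sort order.
; Exposed variables drive that instance's luminance, saturation, hue shift, UV offset, scale and color tint, allowing per-placement variation.
; The event graph holds no runtime logic.
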(fn `UserConstructionScript`
  (bind _decal (`self.Decal`))
  (bind _decal_2 (`self.Decal`))
  (`DecalComponent.SetDecalMaterial` _decal (`self.Decal Material`))
  (bind _returnvalue (`KismetMaterialLibrary.CreateDynamicMaterialInstance` (`DecalComponent.GetDecalMaterial` _decal)))
  (`DecalComponent.SetSortOrder` _decal_2 (`self.Sort Order`))
  (`DecalComponent.SetDecalMaterial` _decal_2 _returnvalue)
  (`MaterialInstanceDynamic.SetScalarParameterValue` _returnvalue "Lum" (`self.Lum`))
  (`MaterialInstanceDynamic.SetScalarParameterValue` _returnvalue "Saturation" (`self.Saturation`))
  (`MaterialInstanceDynamic.SetScalarParameterValue` _returnvalue "Hue Shift" (`self.Hue Shift`))
  (`MaterialInstanceDynamic.SetScalarParameterValue` _returnvalue "Offset X" (`self.Offset X`))
  (`MaterialInstanceDynamic.SetScalarParameterValue` _returnvalue "Offset Y" (`self.Offset Y`))
  (`MaterialInstanceDynamic.SetScalarParameterValue` _returnvalue "Scale X" (`self.Scale X`))
  (`MaterialInstanceDynamic.SetScalarParameterValue` _returnvalue "Scale Y" (`self.Scale Y`))
  (`MaterialInstanceDynamic.SetVectorParameterValue` _returnvalue "Color Tint" (`self.Color Tint`)))