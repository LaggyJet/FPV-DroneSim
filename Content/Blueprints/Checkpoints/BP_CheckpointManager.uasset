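; Checkpoint manager for a drone game that tracks the checkpoint nearest the player and ends the game when none remain.
; BeginPlay gathers all Checkpoint actors and selects the closest by horizontal distance, reselecting whenever the ReachedCheckpoint flag is set.
; Otherwise, Tick prints the distance to that checkpoint as debug output.
; An empty list triggers a one-time finish: game-instance flags, finish menu, UI-only input and visible cursor.
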(event `self.ReceiveTick`
  (params (DeltaSeconds :type "Float (single-precision)"))
  (bind _returnvalue (`GameplayStatics.GetPlayerController` 0))
  (`|ExecutionSequence`
    (:`then_0`
      (if (`self.ReachedCheckpoint`)
        (`self.SetNewCheckpoint`)
        (set `self.ReachedCheckpoint` false)
        (else
          (`self.temp`))))
    (:`then_1`
      (if (== (`KismetArrayLibrary.Array_Length` (`self.Checkpoints`)) 0)
        (`/Engine/EditorBlueprintResources/StandardMacros.DoOnce` false
          (:`Completed`
            (bind _asdrone_game_instance (cast `/Game/Blueprints/DroneGameInstance` (`GameplayStatics.GetGameInstance`)))
            (`Widget.SetVisibility` (`/Game/Blueprints/DroneGameInstance.FinishGameMenuRef` _asdrone_game_instance) "Visible")
            (set `/Game/Blueprints/DroneGameInstance.IsGameFinished` true _asdrone_game_instance)
            (set `/Game/Blueprints/DroneGameInstance.IsGamePaused` true _asdrone_game_instance)
            (`WidgetBlueprintLibrary.SetInputMode_UIOnlyEx` _returnvalue null)
            (set `PlayerController.bShowMouseCursor` true _returnvalue)))))))

(event `self.ReceiveBeginPlay`
  (bind _outactors (`GameplayStatics.GetAllActorsOfClass` "/Game/Blueprints/Checkpoints/Checkpoint.Checkpoint_C"))
  (set `self.Checkpoints` _outactors)
  (`self.SetNewCheckpoint`))

(event `SetNewCheckpoint`
  (for _array_element (`self.Checkpoints`)
    (bind _returnvalue (`self.GetHorizontalDistanceTo` _array_element (`GameplayStatics.GetPlayerPawn` 0)))
    (if (or (< _returnvalue (`self.ClosestDist`)) (not (`KismetSystemLibrary.IsValid` (`self.ClosestCheckpoint`))))
      (set `self.ClosestCheckpoint` _array_element)
      (set `self.ClosestDist` _returnvalue))))

(event `temp`
  (bind _closestcheckpoint (`self.ClosestCheckpoint`))
  (`/Engine/EditorBlueprintResources/StandardMacros.IsValid` _closestcheckpoint
    (:`Is Valid`
      (`KismetSystemLibrary.PrintString` (`KismetStringLibrary.Conv_DoubleToString` (`self.GetHorizontalDistanceTo` _closestcheckpoint (`GameplayStatics.GetPlayerPawn` 0)))))))

(fn `UserConstructionScript`)