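; Checkpoint actor that shows scan state through its material and removes itself when the checkpoint manager's completed scan names it as the closest.
; Any overlap on its Sphere applies the not-started material and binds to the player pawn's ScanSurrounding scan-start event, which switches to the started material.
; Tick polls BP_CheckpointManager; on a match, the checkpoint flags itself reached, leaves the manager's list, self-destructs and resets the scan state.
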(event `self.ReceiveBeginPlay`)

(event `self.ReceiveTick`
  (params (DeltaSeconds :type "Float (single-precision)"))
  (bind _returnvalue (`GameplayStatics.GetActorOfClass` "/Game/Blueprints/Checkpoints/BP_CheckpointManager.BP_CheckpointManager_C"))
  (if (`|EnumEquality` (`CheckpointManager.ScanState` _returnvalue) "Completed")
    (if (== (`/Game/Blueprints/Checkpoints/BP_CheckpointManager.ClosestCheckpoint` _returnvalue) self)
      (set `/Game/Blueprints/Checkpoints/BP_CheckpointManager.ReachedCheckpoint` true _returnvalue)
      (`KismetArrayLibrary.Array_RemoveItem` (`/Game/Blueprints/Checkpoints/BP_CheckpointManager.Checkpoints` _returnvalue) self)
      (set `/Game/Blueprints/Checkpoints/BP_CheckpointManager.ClosestCheckpoint` null _returnvalue)
      (`self.K2_DestroyActor`)
      (set `CheckpointManager.ScanState` "NotStarted" _returnvalue))))

(event `self.Sphere.OnComponentBeginOverlap`
  (params (OverlappedComponent :type "PrimitiveComponent Object Reference") (OtherActor :type "Actor Object Reference") (OtherComp :type "PrimitiveComponent Object Reference") (OtherBodyIndex :type Integer) (bFromSweep :type Boolean) (SweepResult :type "HitResult Structure (by ref)"))
  (`PrimitiveComponent.SetMaterial` (`self.Sphere1`) 0 "/Game/Blueprints/Checkpoints/NotStartedMat.NotStartedMat")
  (add `ScanSurrounding.OnScanStart` (`self.GetComponentByClass` (`GameplayStatics.GetPlayerPawn` 0) "/Script/FPVDroneSim.ScanSurrounding") (delegate `ScanStarted`)))

(event `ScanStarted`
  (`PrimitiveComponent.SetMaterial` (`self.Sphere1`) 0 "/Game/Blueprints/Checkpoints/StartedMat.StartedMat"))

(fn `UserConstructionScript`)